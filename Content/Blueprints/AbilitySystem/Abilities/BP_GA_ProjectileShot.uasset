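; Gameplay ability that fires a rocket projectile from the equipped weapon.
; On activation it traces from weapon to focus and plays weapon effects with a rebuilt hit result lacking a physical material, skipping impact effects in favor of the explosion.
; It launches the rocket along the trace direction, offset from the muzzle to avoid exploding on the shooter, with the character as owner and instigator, then ends immediately.
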(event `self.K2_ActivateAbility`
  (bind _returnvalue (`self.GetActionGameCharacterFromActorInfo`))
  (bind (_bblockinghit _binitialoverlap _time _distance _location _impactpoint _normal _impactnormal _physmat _hitactor _hitcomponent _hitbonename _bonename _hititem _elementindex _faceindex _tracestart _traceend) (`GameplayStatics.BreakHitResult` (`self.GetWeaponToFocusTraceResult` (`WeaponStaticData.ShootingDistance` (`self.GetEquippedItemWeaponStaticData`)) "TraceTypeQuery3")))
  (bind _returnvalue_2 (`KismetMathLibrary.Normal` (- _traceend _tracestart)))
  (`WeaponItemActor.PlayWeaponEffects` (`self.GetEquippedWeaponItemActor`) (`GameplayStatics.MakeHitResult` _bblockinghit _binitialoverlap _time _distance _location _impactpoint _normal _impactnormal null null null "None" "None" 0 0 0 _tracestart _traceend))
  (`ActionGameStatics.LaunchProjectile` "/Game/Blueprints/Projectile/Rocket.Rocket_C" (`KismetMathLibrary.MakeTransform` (+ (`WeaponItemActor.GetMuzzleLocation` (`self.GetEquippedWeaponItemActor`)) (* _returnvalue_2 (`self.SpawnOffset`))) (`KismetMathLibrary.Conv_VectorToRotator` _returnvalue_2)) _returnvalue _returnvalue)
  (`self.K2_EndAbility`))